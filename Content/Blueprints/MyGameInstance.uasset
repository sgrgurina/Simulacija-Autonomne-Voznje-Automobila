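; Game instance that owns a neuroevolution training population of neural networks and a genetic algorithm.
; On Init it builds one single-hidden-layer net per population slot with a matching error value, then configures the algorithm with mutation and elitism.
; Callers report per-net errors by index, GAStep evolves the nets from those errors and logs the training step and best error.
; GetBestNet returns the lowest-error net.
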(event EventInit
  ;[1 1 1] Init nets and errors
  (for _index (range 1 (Variables|Default|GetpopulationSize))
    (bind _returnvalue (Game|ConstructObjectfromClass "/Script/AutonomousCar.NeuralNet" "MyGameInstance"))
    (Class|NeuralNet|InitNet _returnvalue 1 8 9 2 true)
    (Utilities|Array|Add (Variables|Default|GetNets) _returnvalue)
    (Utilities|Array|Add (Variables|Default|GetErrrorValues) 0.0)
    (Development|PrintString "Net Added to Game Instance" false true "(R=0.000000,G=0.660000,B=1.000000,A=1.000000)" 5.0)
    (Class|NeuralNet|PrintNeuronWeights _returnvalue))
  ;[1 1 1] Construct GA
  (bind _returnvalue_2 (Game|ConstructObjectfromClass "/Script/AutonomousCar.GeneticAlgorithm" "MyGameInstance"))
  (bind _output_get (Variables|Default|SetGA _returnvalue_2))
  (Class|GeneticAlgorithm|SetProperties _output_get 0.2 0.8 (Variables|Default|GetpopulationSize) 4)
  (Development|PrintString "Game instance Init complete" true true "(R=0.054143,G=0.760000,B=0.000000,A=1.000000)" 5.0))

(fn GAStep
  (Class|GeneticAlgorithm|Step (Variables|Default|GetGA) (Variables|Default|GetNets) (Variables|Default|GetErrrorValues))
  ;[1 1 1] Print traning step and minimum error value
  (Development|PrintString (Utilities|String|Append "Training Step:" (Utilities|String|ToString(Integer) (Variables|Default|GetTrainingStep))) true true "(R=0.000000,G=0.660000,B=1.000000,A=1.000000)" 5.0)
  (bind __minerror (CallFunction|MinimumError))
  (Development|PrintString (Utilities|String|Append "Best Error Value" (Utilities|String|ToString(Float) __minerror)) true true "(R=0.000000,G=0.660000,B=1.000000,A=1.000000)" 5.0)
  (Math|Integer|IncrementInt (Variables|Default|GetTrainingStep)))

(fn SetErrorValue
  (params (NetIndex :type Integer) (ErrorValue :type Float%20%28single-precision%29))
  (if (< NetIndex (Variables|Default|GetpopulationSize))
    (Utilities|Array|SetArrayElem (Variables|Default|GetErrrorValues) NetIndex ErrorValue)
    (else
      (Development|PrintString "Invalid index for error value"))))

(fn GetBestNet
  (LocalVariables|SetIndexOfBest 0)
  (LocalVariables|SetMinError (Utilities|Array|Get(acopy) (Variables|Default|GetErrrorValues)))
  ;[1 1 1] Find Index of best net
  (for (_array_element _array_index) (Variables|Default|GetErrrorValues)
    (if (< _array_element (LocalVariables|GetMinError))
      (LocalVariables|SetMinError _array_element)
      (LocalVariables|SetIndexOfBest _array_index)))
  ;[1 1 1] Return best net
  (return (Utilities|Array|Get(acopy) (Variables|Default|GetNets) (LocalVariables|GetIndexOfBest))))

(fn MinimumError
  (LocalVariables|SetMinError (Utilities|Array|Get(acopy) (Variables|Default|GetErrrorValues)))
  ;[1 1 1] Find Index of best net
  (for _array_element (Variables|Default|GetErrrorValues)
    (if (< _array_element (LocalVariables|GetMinError))
      (LocalVariables|SetMinError _array_element)))
  (return (LocalVariables|GetMinError)))