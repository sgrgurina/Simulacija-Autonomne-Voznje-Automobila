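; Vehicle pawn that drives a generated track by player input or neural network, with genetic-algorithm training.
; Seven line-trace distance sensors and forward speed feed the net, which outputs throttle and steering.
; Finishing, reversing over the line, hitting rails or moving too slowly ends a lap, scores error and respawns the car.
; Training cycles the game instance's nets, calling GAStep per generation; keybinds also toggle data recording and save or load nets.
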(event OnComponentBeginOverlap(Mesh)
  (params (OverlappedComponent :type Primitive%20Component%20Object%20Reference) (OtherActor :type Actor%20Object%20Reference) (OtherComp :type Primitive%20Component%20Object%20Reference) (OtherBodyIndex :type Integer) (bFromSweep :type Boolean) (SweepResult :type Hit%20Result%20Structure%20%28by%20ref%29))
  ;[1 1 1] Detecting car hitting a guard rail
  (if (Utilities|Enum|Equal(Enum) (Collision|GetCollisionObjectType OtherComp) "ECC_GameTraceChannel1")
    ;[1 1 1] For testing - shows distance traveled upon hitting track
    (bind _distance (Default|ApproximateDistanceAlongTrack (Variables|Default|GetTrack) (Transformation|GetWorldLocation (Variables|Character|GetMesh))))
    (Development|PrintString (Utilities|String|Append "Distance: " (Utilities|String|ToString(Integer) (Math|Float|Truncate _distance)) " Hit: " (Utilities|GetDisplayName OtherComp)) false false "(R=0.000000,G=0.660000,B=1.000000,A=1.000000)" 5.0)
    (CallFunction|TrackHit)))

(event Custom|Lap%20Finished
  (params (LapCompleted :type Boolean))
  ;[1 1 1] Events that react to hitting the finish line
  (if LapCompleted
    (CallFunction|LapCompleted)
    (else
      (CallFunction|FinishLineHitBackwards))))

(event Custom|LapCompleted
  ;[1 1 1] Lap ending events
  (CallFunction|StopLapTime)
  ;[1 1 1] Set distance traveled based on event
  (bind _tracklength (Default|GetTrackLength (Variables|Default|GetTrack)))
  (Variables|Default|SetDistanceTraveled _tracklength)
  (Development|PrintString "Lap Completed" false false "(R=1.000000,G=0.922361,B=0.000000,A=1.000000)" 5.0)
  (bind _returnvalue (Class|NeuralNet|Error (Variables|Default|GetNet) (Variables|Default|GetDistanceTraveled) (Variables|Default|GetTrackLength) (Variables|Default|GetLapTime)))
  (Utilities|FlowControl|Sequence
    (:then_0
      (if (Variables|Default|GetTraining)
        (CallFunction|EndOfTrainingLap _returnvalue)))
    (:then_1
      ;[1 1 1] Information for testing
      (CallFunction|PrintPercentageOfTrackNotReached)
      (CallFunction|PrintSpeedErrorModifier)
      (Development|PrintString (Utilities|String|Append "Error value: " (Utilities|String|ToString(Float) _returnvalue)) true true "(R=0.000000,G=0.660000,B=1.000000,A=1.000000)" 5.0))
    (:then_2
      (CallFunction|StartNewLap))))

(event Custom|Moved%20too%20slow
  ;[1 1 1] Lap ending events
  (CallFunction|StopLapTime)
  ;[1 1 1] Set distance traveled based on event
  (Development|PrintString "Moved too slow" false false "(R=1.000000,G=0.859266,B=0.014152,A=1.000000)" 5.0)
  (bind _distance (Default|ApproximateDistanceAlongTrack (Variables|Default|GetTrack) (Transformation|GetWorldLocation (Variables|Character|GetMesh))))
  (Variables|Default|SetDistanceTraveled _distance)
  (bind _returnvalue (Class|NeuralNet|Error (Variables|Default|GetNet) (Variables|Default|GetDistanceTraveled) (Variables|Default|GetTrackLength) (Variables|Default|GetLapTime)))
  (Utilities|FlowControl|Sequence
    (:then_0
      (if (Variables|Default|GetTraining)
        (CallFunction|EndOfTrainingLap _returnvalue)))
    (:then_1
      ;[1 1 1] Information for testing
      (CallFunction|PrintPercentageOfTrackNotReached)
      (CallFunction|PrintSpeedErrorModifier)
      (Development|PrintString (Utilities|String|Append "Error value: " (Utilities|String|ToString(Float) _returnvalue)) true true "(R=0.000000,G=0.660000,B=1.000000,A=1.000000)" 5.0))
    (:then_2
      (CallFunction|StartNewLap))))

(event Custom|Net%20loaded%20from%20save
  (Variables|Default|SetNetControlled true)
  (CallFunction|StartNewLap))

(event Custom|ResetTimer
  ;[1 1 1] Reset timer
  (Development|PrintString "Reset timer" false false "(R=0.000000,G=1.000000,B=0.017753,A=1.000000)")
  (Utilities|Time|SetTimerbyFunctionName 0 "CheckIfCarIsTooSlow" 1e+01 true))

(event Custom|FinishLineHitBackwards
  ;[1 1 1] Lap ending events
  (CallFunction|StopLapTime)
  ;[1 1 1] Set distance traveled based on event
  (Variables|Default|SetDistanceTraveled 0.0)
  (Development|PrintString "Finish hit backwards" false false "(R=1.000000,G=0.859266,B=0.014152,A=1.000000)" 5.0)
  (bind _returnvalue (Class|NeuralNet|Error (Variables|Default|GetNet) (Variables|Default|GetDistanceTraveled) (Variables|Default|GetTrackLength) (Variables|Default|GetLapTime)))
  (Utilities|FlowControl|Sequence
    (:then_0
      (if (Variables|Default|GetTraining)
        (CallFunction|EndOfTrainingLap _returnvalue)))
    (:then_1
      ;[1 1 1] Information for testing
      (CallFunction|PrintPercentageOfTrackNotReached)
      (CallFunction|PrintSpeedErrorModifier)
      (Development|PrintString (Utilities|String|Append "Error value: " (Utilities|String|ToString(Float) _returnvalue)) true true "(R=0.000000,G=0.660000,B=1.000000,A=1.000000)" 5.0))
    (:then_2
      (CallFunction|StartNewLap))))

(event Custom|ResetLapTime
  ;[1 1 1] Lap timing
  (bind _time (Timeline|LapTimeline PlayFromStart)
    (:Update
      (bind _output_get (Variables|Default|SetLapTime _time)))))

(event Custom|StopLapTime
  ;[1 1 1] Lap timing
  (bind _time (Timeline|LapTimeline Stop)
    (:Update
      (bind _output_get (Variables|Default|SetLapTime _time)))))

(event Custom|TrackHit
  ;[1 1 1] Lap ending events
  (CallFunction|StopLapTime)
  ;[1 1 1] Set distance traveled based on event
  (Development|PrintString "Track hit" false false "(R=1.000000,G=0.928630,B=0.063832,A=1.000000)" 5.0)
  (bind _distance (Default|ApproximateDistanceAlongTrack (Variables|Default|GetTrack) (Transformation|GetWorldLocation (Variables|Character|GetMesh))))
  (Variables|Default|SetDistanceTraveled _distance)
  (bind _returnvalue (Class|NeuralNet|Error (Variables|Default|GetNet) (Variables|Default|GetDistanceTraveled) (Variables|Default|GetTrackLength) (Variables|Default|GetLapTime)))
  (Utilities|FlowControl|Sequence
    (:then_0
      (if (Variables|Default|GetTraining)
        (CallFunction|EndOfTrainingLap _returnvalue)))
    (:then_1
      ;[1 1 1] Information for testing
      (CallFunction|PrintPercentageOfTrackNotReached)
      (CallFunction|PrintSpeedErrorModifier)
      (Development|PrintString (Utilities|String|Append "Error value: " (Utilities|String|ToString(Float) _returnvalue)) true true "(R=0.000000,G=0.660000,B=1.000000,A=1.000000)" 5.0))
    (:then_2
      (CallFunction|StartNewLap))))

(event Custom|Start%20new%20lap
  ;[1 1 1] Starting a new lap
  (CallFunction|StopCar)
  (CallFunction|Respawn)
  ;;[1 1 1] Wait for car to completely stop
  (Utilities|FlowControl|Delay 0.4)
  (CallFunction|StartCar)
  (CallFunction|ResetLapTime)
  (CallFunction|ResetTimer)
  (Variables|Default|SetLastDistanceTraveled 0.0))

(event EventBeginPlay
  (Utilities|FlowControl|Sequence
    (:then_0
      (if (Variables|Default|GetUsingNewNet)
        (CallFunction|InitNewNet)))
    (:then_1
      (CallFunction|SetUpTrack))
    (:then_2
      ;[1 1 1] Events that react to hitting the finish line
      (EventDispatchers|BindEventtoFinishLineDispatcher (Variables|Default|GetTrack) (delegate Custom|Lap%20Finished)))
    (:then_3
      ;[1 1 1] Lap timing
      (bind _time (Timeline|LapTimeline PlayFromStart)
        (:Update
          (bind _output_get (Variables|Default|SetLapTime _time)))))
    (:then_4
      ;[1 1 1] Reset timer
      (Utilities|Time|SetTimerbyFunctionName 0 "CheckIfCarIsTooSlow" 1e+01 true))
    (:then_5
      ;[1 1 1] Sensor reading display
      (bind _returnvalue (AddComponent|AddTextRenderComponent false (Math|Transform|MakeTransform "0, 0,150.000000" "0.000000,180.000000,0.000000" "1.000000,1,1")))
      (bind _returnvalue_2 (AddComponent|AddTextRenderComponent false (Math|Transform|MakeTransform "0.000000,-300.000000,100.000000" "0.000000,180.000000,0.000000" "1.000000,1,1")))
      (bind _returnvalue_3 (AddComponent|AddTextRenderComponent false (Math|Transform|MakeTransform "0,300.000000,100.000000" "0.000000,180.000000,0.000000" "1.000000,1,1")))
      (bind _returnvalue_4 (AddComponent|AddTextRenderComponent false (Math|Transform|MakeTransform "0,-100.000000,150.000000" "0.000000,180.000000,0.000000" "1.000000,1,1")))
      (bind _returnvalue_5 (AddComponent|AddTextRenderComponent false (Math|Transform|MakeTransform "0,100.000000,150.000000" "0.000000,180.000000,0.000000" "1.000000,1,1.000000")))
      (bind _returnvalue_6 (AddComponent|AddTextRenderComponent false (Math|Transform|MakeTransform "0,-200.000000,150.000000" "0.000000,180.000000,0.000000" "1.000000,1,1")))
      (bind _returnvalue_7 (AddComponent|AddTextRenderComponent false (Math|Transform|MakeTransform "0,200.000000,150.000000" "0.000000,180.000000,0.000000" "1.000000,1,1"))))))

(event EventTick
  (params (DeltaSeconds :type Float%20%28single-precision%29))
  (Utilities|FlowControl|Sequence
    (:then_0
      ;[1 1 1] Do sensor readings
      (bind _sensor_distance (CallFunction|GetDistancefromSensor (Variables|Default|GetFrontSensorBox)))
      (bind _output_get (Variables|Default|SetCenterSensorDist _sensor_distance))
      ;[1 1 1] Sensor reading display
      (Rendering|Components|TextRender|SetText (stale EventBeginPlay _returnvalue) (Utilities|Text|ToText(String) (Utilities|String|ToString(Integer) (Math|Float|Ceil _output_get)))))
    (:then_1
      (bind _sensor_distance_2 (CallFunction|GetDistancefromSensor (Variables|Default|GetFarLeftSensorBox)))
      (bind _output_get_2 (Variables|Default|SetFarLeftSensorDist _sensor_distance_2))
      (Rendering|Components|TextRender|SetText (stale EventBeginPlay _returnvalue_2) (Utilities|Text|ToText(String) (Utilities|String|ToString(Integer) (Math|Float|Ceil _output_get_2)))))
    (:then_2
      (bind _sensor_distance_3 (CallFunction|GetDistancefromSensor (Variables|Default|GetFarRightSensorBox)))
      (bind _output_get_3 (Variables|Default|SetFarRightSensorDist _sensor_distance_3))
      (Rendering|Components|TextRender|SetText (stale EventBeginPlay _returnvalue_3) (Utilities|Text|ToText(String) (Utilities|String|ToString(Integer) (Math|Float|Ceil _output_get_3)))))
    (:then_3
      (bind _sensor_distance_4 (CallFunction|GetDistancefromSensor (Variables|Default|GetCloseLeftSensorBox)))
      (bind _output_get_4 (Variables|Default|SetCloseLeftSensorDist _sensor_distance_4))
      (Rendering|Components|TextRender|SetText (stale EventBeginPlay _returnvalue_4) (Utilities|Text|ToText(String) (Utilities|String|ToString(Integer) (Math|Float|Ceil _output_get_4)))))
    (:then_4
      (bind _sensor_distance_5 (CallFunction|GetDistancefromSensor (Variables|Default|GetCloseRightSensorBox)))
      (bind _output_get_5 (Variables|Default|SetCloseRightSensorDist _sensor_distance_5))
      (Rendering|Components|TextRender|SetText (stale EventBeginPlay _returnvalue_5) (Utilities|Text|ToText(String) (Utilities|String|ToString(Integer) (Math|Float|Ceil _output_get_5)))))
    (:then_5
      (bind _sensor_distance_6 (CallFunction|GetDistancefromSensor (Variables|Default|GetMiddleLeftSensorBox)))
      (bind _output_get_6 (Variables|Default|SetMiddleLeftSensorDist _sensor_distance_6))
      (Rendering|Components|TextRender|SetText (stale EventBeginPlay _returnvalue_6) (Utilities|Text|ToText(String) (Utilities|String|ToString(Integer) (Math|Float|Ceil _output_get_6)))))
    (:then_6
      (bind _sensor_distance_7 (CallFunction|GetDistancefromSensor (Variables|Default|GetMiddleRightSensorBox)))
      (bind _output_get_7 (Variables|Default|SetMiddleRightSensorDist _sensor_distance_7))
      (Rendering|Components|TextRender|SetText (stale EventBeginPlay _returnvalue_7) (Utilities|Text|ToText(String) (Utilities|String|ToString(Integer) (Math|Float|Ceil _output_get_7)))))
    (:then_7
      (if (Variables|Default|GetRecording)
        ;[1 1 1] Writes sensor data and speed  to file
        (Class|MyCar|WritetoFile (Class|WheeledVehicleMovementComponent|GetForwardSpeed (Variables|Default|GetVehicleMovement)))))
    (:then_8
      ;[1 1 1] Whether neural net controls the car
      (if (Variables|Default|GetNetControlled)
        (CallFunction|PassNetOutputstoCarInput)))))

(event Input|ActionEvents|InputActionSave
  (params (Key :type Key%20Structure :default "AnyKey"))
  ;[1 1 1] Save game
  (:Pressed
    (Development|PrintString "Game saving" true true "(R=0.995000,G=0.248446,B=0.000000,A=1.000000)" 5.0)
    (bind _returnvalue (SaveGame|CreateSaveGameObject "/Game/Blueprints/NetSaveGame.NetSaveGame_C"))
    (CallFunction|SaveNeuralNet _returnvalue)
    (bind _returnvalue_2 (SaveGame|SaveGametoSlot _returnvalue "Quicksave"))
    (if _returnvalue_2
      (Development|PrintString "Saved successfully" true true "(R=1.000000,G=0.756870,B=0.000000,A=1.000000)")
      (Class|NeuralNet|PrintNeuronWeights (Variables|Default|GetNet))
      (CallFunction|StartNewLap)
      (else
        (Development|PrintString "Save failed")))))

(event Input|ActionEvents|InputActionDebugvehiclecommand
  (params (Key :type Key%20Structure :default "AnyKey"))
  ;[1 1 1] Debug screen keybind
  (:Pressed
    (Development|ExecuteConsoleCommand "showdebug vehicle")))

(event Input|ActionEvents|InputActionRecording
  (params (Key :type Key%20Structure :default "AnyKey"))
  ;[1 1 1] Data recording keybind
  (:Pressed
    (Variables|Default|Setrecording (not (Variables|Default|Getrecording)))))

(event Input|ActionEvents|InputActionStartTraining
  (params (Key :type Key%20Structure :default "AnyKey"))
  ;[1 1 1] Training keybinds
  (:Pressed
    (CallFunction|StartTraining)))

(event Input|ActionEvents|InputActionStopTraining
  (params (Key :type Key%20Structure :default "AnyKey"))
  ;[1 1 1] Training keybinds
  (:Pressed
    (Variables|Default|SetTrainingStopped true)))

(event Input|ActionEvents|InputActionLoad
  (params (Key :type Key%20Structure :default "AnyKey"))
  ;[1 1 1] Load game
  (:Pressed
    (bind _returnvalue (SaveGame|DoesSaveGameExist "Quicksave"))
    (if _returnvalue
      (bind _returnvalue_2 (SaveGame|LoadGamefromSlot "Quicksave"))
      (bind _asnet_save_game (Utilities|Casting|CastToNetSaveGame _returnvalue_2))
      (CallFunction|LoadNeuralNet _asnet_save_game)
      (if (Utilities|IsValid (Variables|Default|GetNet))
        (Development|PrintString "Net is valid" false)
        (Development|PrintString "Net Loaded" false)
        (Class|NeuralNet|PrintNeuronWeights (Variables|Default|GetNet))
        (CallFunction|NetLoadedfromSave)
        (else
          (Development|PrintString "Net is not valid" false)))
      (else
        (Development|PrintString "Save does not exist" true true "(R=1.000000,G=0.000000,B=0.000000,A=1.000000)" 5.0)))))

(event Input|AxisEvents|InputAxisForward
  (params (AxisValue :type Float%20%28single-precision%29))
  ;[1 1 1] Pass inputs to vehicle
  (Class|WheeledVehicleMovementComponent|SetThrottleInput (Variables|Default|GetVehicleMovement) AxisValue)
  (Variables|Default|SetThrottleValue AxisValue))

(event Input|AxisEvents|InputAxisRight
  (params (AxisValue :type Float%20%28single-precision%29))
  ;[1 1 1] Pass inputs to vehicle
  (Class|WheeledVehicleMovementComponent|SetSteeringInput (Variables|Default|GetVehicleMovement) AxisValue)
  (Variables|Default|SetSteeringValue AxisValue))

(fn ConstructionScript)

(fn GetDistancefromSensor
  (params (Sensor :type Box%20Component%20Object%20Reference))
  (bind _returnvalue (Transformation|GetWorldLocation Sensor))
  (bind _returnvalue_2 (Transformation|GetWorldRotation Sensor))
  (bind _returnvalue_3 (Math|Vector|GetForwardVector _returnvalue_2))
  (bind _returnvalue_4 (* _returnvalue_3 3e+04))
  (bind _returnvalue_5 (+ _returnvalue _returnvalue_4))
  (bind (_x _y) (Math|Vector|BreakVector _returnvalue_5))
  (bind _outhit (Collision|LineTraceForObjects _returnvalue (Math|Vector|MakeVector _x _y (.Z (Math|Vector|BreakVector _returnvalue))) (Utilities|Array|MakeArray "ObjectTypeQuery7") false 0 "ForOneFrame"))
  (return (Math|Vector|VectorLength (- (.ImpactPoint (Collision|BreakHitResult _outhit)) (Transformation|GetWorldLocation Sensor)))))

(fn PassNetOutputstoCarInput
  (bind _vehiclemovement (Variables|Default|GetVehicleMovement))
  ;[1 1 1] Get net output
  (bind _returnvalue (Class|NeuralNet|Output (Variables|Default|GetNet) (Utilities|Array|MakeArray (Variables|Default|GetCenterSensorDist) (Variables|Default|GetCloseLeftSensorDist) (Variables|Default|GetCloseRightSensorDist) (Variables|Default|GetMiddleLeftSensorDist) (Variables|Default|GetMiddleRightSensorDist) (Variables|Default|GetFarLeftSensorDist) (Variables|Default|GetFarRightSensorDist) (Class|WheeledVehicleMovementComponent|GetForwardSpeed (Variables|Default|GetVehicleMovement)))))
  (Utilities|FlowControl|Sequence
    (:then_0
      ;[1 1 1] Set vehicle throttle and steering
      (bind _output_get (Variables|Default|SetThrottleValue (Utilities|Array|Get(acopy) _returnvalue)))
      (Class|WheeledVehicleMovementComponent|SetThrottleInput _vehiclemovement _output_get))
    (:then_1
      (bind _output_get_2 (Variables|Default|SetSteeringValue (Utilities|Array|Get(acopy) _returnvalue 1)))
      (Class|WheeledVehicleMovementComponent|SetSteeringInput _vehiclemovement _output_get_2))))

(fn InitNewNet
  (bind _returnvalue (Game|ConstructObjectfromClass "/Script/AutonomousCar.NeuralNet" "MyCar"))
  (bind _output_get (Variables|Default|SetNet _returnvalue))
  (Class|NeuralNet|InitNet _output_get 1 8 9 2 true)
  (Class|NeuralNet|PrintNeuronWeights (Variables|Default|GetNet)))

(fn Respawn
  (Transformation|SetActorLocation (Transformation|GetWorldLocation (Variables|/Game/Blueprints/TrackGenerator.TrackGenerator_C|GetSpawnPoint (Variables|Default|GetTrack))) false true)
  (Transformation|SetActorRotation (Transformation|GetWorldRotation (Variables|/Game/Blueprints/TrackGenerator.TrackGenerator_C|GetSpawnPoint (Variables|Default|GetTrack))) true))

(fn PrintPercentageOfTrackNotReached
  (bind _tracklength (Variables|Default|GetTrackLength))
  (Development|PrintString (Utilities|String|Append "Percentage not reached: " (Utilities|String|ToString(Float) (* (/ (- _tracklength (Variables|Default|GetDistanceTraveled)) _tracklength) 1e+02))) false true "(R=0.000000,G=0.049669,B=0.750000,A=1.000000)" 1e+01))

(fn PrintSpeedErrorModifier
  (bind _distancetraveled (Variables|Default|GetDistanceTraveled))
  ;[1 1 1] Was distance traveled 0
  (if (== _distancetraveled 0.0)
    (Development|PrintString "Speed error modifier: infinite" true false "(R=1.000000,G=0.000000,B=0.000000,A=1.000000)" 5.0)
    (else
      (Development|PrintString (Utilities|String|Append "Speed error modifier: " (Utilities|String|ToString(Float) (* (/ (Variables|Default|GetLapTime) (/ _distancetraveled 1e+02)) 5e+01))) true false "(R=0.815000,G=0.000000,B=0.000000,A=1.000000)" 5.0))))

(fn CheckifCarIsTooSlow
  (bind _distance (Default|ApproximateDistanceAlongTrack (Variables|Default|GetTrack) (Transformation|GetWorldLocation (Variables|Character|GetMesh))))
  (if (< (/ (- (/ _distance 1e+02) (Variables|Default|GetLastDistanceTraveled)) 1e+01) 3.0)
    (CallFunction|MovedTooSlow)
    (else
      (Variables|Default|SetLastDistanceTraveled (/ _distance 1e+02)))))

(fn SaveNeuralNet
  (params (SaveObject :type Net%20Save%20Game%20Object%20Reference))
  (bind _net (Variables|Default|GetNet))
  (bind _returnvalue (Class|NeuralNet|GetNumOfInputs _net))
  (Variables|/Game/Blueprints/NetSaveGame.NetSaveGame_C|SetInputSize SaveObject _returnvalue)
  (bind _returnvalue_2 (Class|NeuralNet|GetHiddenLayerSize _net))
  (Variables|/Game/Blueprints/NetSaveGame.NetSaveGame_C|SetLayerSize SaveObject _returnvalue_2)
  (bind _returnvalue_3 (Class|NeuralNet|GetNumOfHiddenLayers _net))
  (Variables|/Game/Blueprints/NetSaveGame.NetSaveGame_C|SetNumOfHiddenLayers SaveObject _returnvalue_3)
  (bind _returnvalue_4 (Class|NeuralNet|GetNumOfOutputs _net))
  (Variables|/Game/Blueprints/NetSaveGame.NetSaveGame_C|SetOutputSize SaveObject _returnvalue_4)
  (bind _returnvalue_5 (Class|NeuralNet|GetFlatWeights _net))
  (Variables|/Game/Blueprints/NetSaveGame.NetSaveGame_C|SetWeights SaveObject _returnvalue_5)
  (Variables|/Game/Blueprints/NetSaveGame.NetSaveGame_C|SetbiasNeurons SaveObject (Variables|/Script/AutonomousCar.NeuralNet|GethasBiasNeurons _net)))

(fn LoadNeuralNet
  (params (Save :type Net%20Save%20Game%20Object%20Reference))
  (bind _weights (Variables|/Game/Blueprints/NetSaveGame.NetSaveGame_C|GetWeights Save))
  (bind _returnvalue (Game|ConstructObjectfromClass "/Script/AutonomousCar.NeuralNet" "MyCar"))
  (bind _output_get (Variables|Default|SetNet _returnvalue))
  (Class|NeuralNet|InitNetwithWeights _output_get (Variables|/Game/Blueprints/NetSaveGame.NetSaveGame_C|GetNumOfHiddenLayers Save) (Variables|/Game/Blueprints/NetSaveGame.NetSaveGame_C|GetInputSize Save) (Variables|/Game/Blueprints/NetSaveGame.NetSaveGame_C|GetLayerSize Save) (Variables|/Game/Blueprints/NetSaveGame.NetSaveGame_C|GetOutputSize Save) (Variables|/Game/Blueprints/NetSaveGame.NetSaveGame_C|GetbiasNeurons Save) _weights)
  (Development|PrintString "Loaded Weights:")
  (for _array_element _weights
    (Development|PrintString (Utilities|String|ToString(Float) _array_element) false)))

(fn SetUpTrack
  ;[1 1 1] Get Track From Scene
  (bind _outactors (Actor|GetAllActorsOfClass "/Game/Blueprints/TrackGenerator.TrackGenerator_C"))
  (bind _output_get (Variables|Default|SetTrack (Utilities|Array|Get(acopy) _outactors)))
  ;[1 1 1] Set Track Length
  (bind _tracklength (Default|GetTrackLength _output_get))
  (bind _output_get_2 (Variables|Default|SetTrackLength _tracklength))
  ;[1 1 1] For testing - print track length
  (Development|PrintString (Utilities|String|Append "Track length: " (Utilities|String|ToString(Float) _output_get_2)) true true "(R=0.000000,G=0.660000,B=1.000000,A=1.000000)" 5.0))

(fn EndOfTrainingLap
  (params (Error :type Float%20%28single-precision%29))
  (Utilities|FlowControl|Sequence
    (:then_0
      ;[1 1 1] Set Error Value For Current Net
      (bind _asmy_game_instance (Utilities|Casting|CastToMyGameInstance (Game|GetGameInstance))
        (:then
          (Default|SetErrorValue _asmy_game_instance (Variables|Default|GetNeuralNetIndex) Error))
        (:CastFailed
          (Development|PrintString "Game Instance Cast Failed"))))
    (:then_1
      ;[1 1 1] Check if that was the last net in the population
      (Math|Integer|IncrementInt (Variables|Default|GetNeuralNetIndex)
        (:%20%20
          (if (== (Variables|/Game/Blueprints/MyGameInstance.MyGameInstance_C|GetpopulationSize _asmy_game_instance) (Variables|Default|GetNeuralNetIndex))
            (bind _asmy_game_instance_2 (Utilities|Casting|CastToMyGameInstance (Game|GetGameInstance)))
            ;[1 1 1] Changes weights
            (Default|GAStep _asmy_game_instance_2)
            (Variables|Default|SetNeuralNetIndex 0)
            (Development|PrintString "Training Step Complete" false false "(R=0.000000,G=0.660000,B=1.000000,A=1.000000)" 5.0)
            (if (Variables|Default|GetTrainingStopped)
              (Variables|Default|SetTraining false)
              ;[1 1 1] Place best net in control of car
              (bind _asmy_game_instance_3 (Utilities|Casting|CastToMyGameInstance (Game|GetGameInstance)))
              (bind _bestnet (Default|GetBestNet _asmy_game_instance_3))
              (Variables|Default|SetNet _bestnet))
            (else
              ;[1 1 1] Change net for next lap
              (bind _asmy_game_instance_4 (Utilities|Casting|CastToMyGameInstance (Game|GetGameInstance)))
              (Variables|Default|SetNet (Utilities|Array|Get(acopy) (Variables|/Game/Blueprints/MyGameInstance.MyGameInstance_C|GetNets _asmy_game_instance_4) (Variables|Default|GetNeuralNetIndex)))
              (Development|PrintString "Next Net Set" false false "(R=0.000000,G=0.660000,B=1.000000,A=1.000000)" 5.0))))))))

(fn StartTraining
  ;[1 1 1] Set first net from population
  (bind _asmy_game_instance (Utilities|Casting|CastToMyGameInstance (Game|GetGameInstance))
    (:then
      (bind _output_get (Variables|Default|SetNet (Utilities|Array|Get(acopy) (Variables|/Game/Blueprints/MyGameInstance.MyGameInstance_C|GetNets _asmy_game_instance))))
      ;[1 1 1] For testing
      (Development|PrintString "Net Loaded From Game Instance" false)
      (Class|NeuralNet|PrintNeuronWeights _output_get)
      (Development|PrintString "Training started")
      (Variables|Default|SetTraining true)
      (CallFunction|StartNewLap))
    (:CastFailed
      (Development|PrintString "Game Instance Cast Failed During Training Start"))))

(fn StopCar
  (if (Variables|Default|GetTraining)
    (Variables|Default|SetNetControlled false))
  (Class|WheeledVehicleMovementComponent|SetHandbrakeInput (Variables|Default|GetVehicleMovement) true)
  (Class|PrimitiveComponent|SetAllPhysicsLinearVelocity (Variables|Character|GetMesh) "0, 0, 0" false))

(fn StartCar
  (Class|WheeledVehicleMovementComponent|SetHandbrakeInput (Variables|Default|GetVehicleMovement) false)
  (if (Variables|Default|GetTraining)
    (Variables|Default|SetNetControlled true)))