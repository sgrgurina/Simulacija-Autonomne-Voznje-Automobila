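; Spline-driven race track generator that builds the road and finish line logic for MyCar.
; The construction script syncs a per-point data array to the spline, then adds spline meshes per segment for road and optional left/right guard rails, wrapping into a closed loop.
; Per-point width, thickness and bank shape each segment.
; Finish line overlaps dispatch crossing direction from a velocity dot product, and helpers report track length and approximate distance along it.
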(event OnComponentBeginOverlap(Finishline)
  (params (OverlappedComponent :type Primitive%20Component%20Object%20Reference) (OtherActor :type Actor%20Object%20Reference) (OtherComp :type Primitive%20Component%20Object%20Reference) (OtherBodyIndex :type Integer) (bFromSweep :type Boolean) (SweepResult :type Hit%20Result%20Structure%20%28by%20ref%29))
  (bind _asmy_car (Utilities|Casting|CastToMyCar OtherActor)
    (:then
      ;[1 1 1] Check if finish line was hit in the right direction
      (if (> (Math|Vector|DotProduct (Transformation|GetVelocity _asmy_car) (Math|Rotator|GetRotationXVector (Transformation|GetWorldRotation (Variables|Default|GetFinish%20line)))) 0.0)
        _
        (else
          _))
      (Default|CallFinishLineDispatcher (> (Math|Vector|DotProduct (Transformation|GetVelocity _asmy_car) (Math|Rotator|GetRotationXVector (Transformation|GetWorldRotation (Variables|Default|GetFinish%20line)))) 0.0)))
    (:CastFailed
      (Development|PrintString "Not MyCar" false))))

(event EventBeginPlay)

(fn ConstructionScript
  (Utilities|FlowControl|Sequence
    (:then_0
      (|SetNumberOfSplinePoints))
    (:then_1
      (|BuildRoadDataArray))
    (:then_2
      (|ConstructionLoop)
      (|StoreDrawGuardRails)
      (Utilities|FlowControl|Sequence
        (:then_0
          ;[1 1 1] Road
          (CallFunction|BuildTrackElement (Variables|Default|GetCurrLoopIndex) (Variables|Default|GetRoadMesh) false))
        (:then_1
          ;[1 1 1] Left guard rail
          (if (Variables|Default|GetDrawLeftGuardRail)
            (CallFunction|BuildTrackElement (Variables|Default|GetCurrLoopIndex) (Variables|Default|GetLeftGuardRailMesh) true)))
        (:then_2
          ;[1 1 1] Right guard rail
          (if (Variables|Default|GetDrawRightGuardRail)
            (CallFunction|BuildTrackElement (Variables|Default|GetCurrLoopIndex) (Variables|Default|GetRightGuardRailMesh) true)))))))

(fn BuildTrackElement
  (params (LoopIndex :type Integer) (TrackElementMesh :type Static%20Mesh%20Object%20Reference) (IsGuardRail :type Boolean))
  ;[1 1 1] Set index for current and next point
  (LocalVariables|SetcurrentLoopIndex LoopIndex)
  (LocalVariables|SetnextLoopIndex (Math|Integer|%(Integer) (+ LoopIndex 1) (Variables|Default|GetSplinePointsNum)))
  (LocalVariables|SettrackElMesh TrackElementMesh)
  (LocalVariables|SetLocal_IsGuardRail IsGuardRail)
  (Utilities|FlowControl|Sequence
    (:then_0
      (LocalVariables|SetstartLocation (.Location (Spline|GetLocationandTangentatSplinePoint (Variables|Default|GetSpline) (LocalVariables|GetcurrentLoopIndex) "Local")))
      (LocalVariables|SetstartTangent (.Tangent (Spline|GetLocationandTangentatSplinePoint (Variables|Default|GetSpline) (LocalVariables|GetcurrentLoopIndex) "Local")))
      (LocalVariables|SetendLocation (.Location (Spline|GetLocationandTangentatSplinePoint (Variables|Default|GetSpline) (LocalVariables|GetnextLoopIndex) "Local")))
      (LocalVariables|SetendTangent (.Tangent (Spline|GetLocationandTangentatSplinePoint (Variables|Default|GetSpline) (LocalVariables|GetnextLoopIndex) "Local")))
      (LocalVariables|SetstartRoll (.trackbank (Utilities|Array|Get(acopy) (Variables|Default|GetRoadDataArray) (LocalVariables|GetcurrentLoopIndex))))
      (LocalVariables|SetstartScale (Math|Vector2D|MakeVector2D (.trackwidth (Utilities|Array|Get(acopy) (Variables|Default|GetRoadDataArray) (LocalVariables|GetcurrentLoopIndex))) (.trackthickness (Utilities|Array|Get(acopy) (Variables|Default|GetRoadDataArray) (LocalVariables|GetcurrentLoopIndex)))))
      (LocalVariables|SetendRoll (.trackbank (Utilities|Array|Get(acopy) (Variables|Default|GetRoadDataArray) (LocalVariables|GetnextLoopIndex))))
      (LocalVariables|SetendScale (Math|Vector2D|MakeVector2D (.trackwidth (Utilities|Array|Get(acopy) (Variables|Default|GetRoadDataArray) (LocalVariables|GetnextLoopIndex))) (.trackthickness (Utilities|Array|Get(acopy) (Variables|Default|GetRoadDataArray) (LocalVariables|GetnextLoopIndex))))))
    (:then_1
      (bind _returnvalue (AddComponent|AddSplineMeshComponent false))
      (bind _output_get (LocalVariables|SetcurrentSplineMesh _returnvalue))
      (Components|StaticMesh|SetStaticMesh _output_get (LocalVariables|GettrackElMesh))
      (SplineMesh|SetStartandEnd (LocalVariables|GetcurrentSplineMesh) (LocalVariables|GetstartLocation) (LocalVariables|GetstartTangent) (LocalVariables|GetendLocation) (LocalVariables|GetendTangent) true :!class /Script/Engine.SplineMeshComponent)
      (Class|SplineMeshComponent|SetStartRoll (LocalVariables|GetcurrentSplineMesh) (LocalVariables|GetstartRoll) true)
      (Class|SplineMeshComponent|SetEndRoll (LocalVariables|GetcurrentSplineMesh) (LocalVariables|GetendRoll) true)
      (SplineMesh|SetStartScale (LocalVariables|GetcurrentSplineMesh) (LocalVariables|GetstartScale) true :!class /Script/Engine.SplineMeshComponent)
      (SplineMesh|SetEndScale (LocalVariables|GetcurrentSplineMesh) (LocalVariables|GetendScale) true :!class /Script/Engine.SplineMeshComponent)
      (Collision|SetCollisionEnabled (LocalVariables|GetcurrentSplineMesh) (select (Variables|Default|GetCollisions) "QueryAndPhysics" "NoCollision"))
      (if (LocalVariables|GetLocal_IsGuardRail)
        (Collision|SetCollisionObjectType (LocalVariables|GetcurrentSplineMesh) "ECC_GameTraceChannel1")))))

(fn ApproximateDistanceAlongTrack
  (params (Location :type Vector))
  (bind _spline (Variables|Default|GetSpline))
  (bind _spline_2 (Variables|Default|GetSpline))
  (bind _returnvalue (Class|SplineComponent|FindInputKeyClosesttoWorldLocation _spline_2 Location))
  (bind _returnvalue_2 (Math|Float|Truncate _returnvalue))
  (bind _returnvalue_3 (Spline|GetDistanceAlongSplineatSplinePoint _spline _returnvalue_2))
  (return (+ _returnvalue_3 (* (- (Spline|GetDistanceAlongSplineatSplinePoint (Variables|Default|GetSpline) (+ _returnvalue_2 1)) _returnvalue_3) (- _returnvalue (Math|Conversions|ToFloat(Integer) _returnvalue_2))))))

(fn GetTrackLength
  (return (Spline|GetSplineLength (Variables|Default|GetSpline))))